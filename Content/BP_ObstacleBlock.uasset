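; BP_ObstacleBlock is an obstacle actor whose static mesh blinks faster over time, apparently signalling its approaching expiration.
; On BeginPlay, an endless Delay loop toggles mesh visibility, starting with an interval of half the expiration time.
; Each cycle cuts that interval to a third, clamped at a minimum, while the second delay stays constant.
; The graph only toggles visibility and never destroys the actor or changes collision.
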(event EventBeginPlay
  (bind _output_get (Variables|Default|SetVisibility%20Off%20Interval (/ (Variables|Default|GetObstacleExpirationTime) 2.0)))
  (Utilities|FlowControl|Delay _output_get :!label _label)
  (Rendering|ToggleVisibility (Variables|Default|GetStaticMesh) false)
  (Utilities|FlowControl|Delay (Variables|Default|GetVisibility%20On%20Interval))
  (Rendering|ToggleVisibility (Variables|Default|GetStaticMesh) false)
  (if (> (/ (Variables|Default|GetVisibility%20Off%20Interval) 3.0) (Variables|Default|GetMinToggleFrequency))
    (Variables|Default|SetVisibility%20Off%20Interval (/ (Variables|Default|GetVisibility%20Off%20Interval) 3.0))
    (goto _label)
    (else
      (Variables|Default|SetVisibility%20Off%20Interval (Variables|Default|GetMinToggleFrequency))
      (goto _label))))

(event Collision|EventActorBeginOverlap
  (params (OtherActor :type Actor%20Object%20Reference)))

(event EventTick
  (params (DeltaSeconds :type Float%20%28single-precision%29)))

(fn ConstructionScript)