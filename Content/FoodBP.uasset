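; Food actor for a snake game, with accelerating and double-score variants shown by swapping the sphere's material.
; On BeginPlay it caches the SnakeBP actor, then blinks the sphere in a delay loop that starts at half the expiration time and speeds up to a minimum interval.
; Each Tick runs a synchronous navigation path query to the snake, prints the result and calls DestroyExpiredFood when the path is invalid.
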(event EventBeginPlay
  (bind _returnvalue (Actor|GetActorOfClass "/Game/SnakeBP.SnakeBP_C"))
  (Variables|Default|SetSnakeRef _returnvalue)
  (if (Variables|Default|GetbIsAccelerating)
    (Rendering|Material|SetMaterial (Variables|Default|GetSphere) 0 "/Engine/VREditor/UI/ArrowMaterial.ArrowMaterial")
    (elif (Variables|Default|GetbIsDoubleScore)
      (Rendering|Material|SetMaterial (Variables|Default|GetSphere) 0 "/Engine/EditorMaterials/WidgetMaterial_Current.WidgetMaterial_Current")))
  (bind _output_get (Variables|Default|SetVisibilityOffInterval (/ (Variables|Default|GetFoodExpirationTime) 2.0)))
  (Utilities|FlowControl|Delay _output_get :!label _label)
  (Rendering|ToggleVisibility (Variables|Default|GetSphere) false)
  (Utilities|FlowControl|Delay (Variables|Default|GetVisibilityOnInterval))
  (Rendering|ToggleVisibility (Variables|Default|GetSphere) false)
  (if (> (/ (Variables|Default|GetVisibilityOffInterval) 3.0) (Variables|Default|GetMinToggleFrequency))
    (Variables|Default|SetVisibilityOffInterval (/ (Variables|Default|GetVisibilityOffInterval) 3.0))
    (goto _label)
    (else
      (Variables|Default|SetVisibilityOffInterval (Variables|Default|GetMinToggleFrequency))
      (goto _label))))

(event EventTick
  (params (DeltaSeconds :type Float%20%28single-precision%29))
  (bind _returnvalue (Class|NavigationSystemV1|FindPathtoActorSynchronously (Transformation|GetActorLocation) (Variables|Default|GetSnakeRef) 5e+01 0 0))
  (if (Utilities|IsValid _returnvalue)
    (Development|PrintString "Path is valid" true true "(R=0.000000,G=0.466667,B=0.018398,A=1.000000)")
    (else
      (Development|PrintString "Path is not valid" true true "(R=0.487500,G=0.020625,B=0.008985,A=1.000000)")
      (Class|Food|DestroyExpiredFood))))

(fn ConstructionScript)